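; BP_LobbyGameMode is the lobby game mode that puts up the lobby UI when play begins.
; With a head-mounted display enabled, it spawns a BP_LobbyWidgetActor at a transform built from the player pawn's forward vector.
; Otherwise it switches the player controller to UI-only input, shows the mouse cursor and adds BP_LobbyWidget to the viewport.
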(event `self.ReceiveBeginPlay`
  (bind _returnvalue (`GameplayStatics.GetPlayerController` 0))
  (if (`HeadMountedDisplayFunctionLibrary.IsHeadMountedDisplayEnabled`)
    (`|SpawnActorFromClass` "/Game/Game/BP_LobbyWidgetActor.BP_LobbyWidgetActor_C" (`KismetMathLibrary.Conv_VectorToTransform` (`self.GetActorForwardVector` (`GameplayStatics.GetPlayerPawn` 0))) "Undefined" "MultiplyWithRoot" null null)
    (else
      (`WidgetBlueprintLibrary.SetInputMode_UIOnlyEx` _returnvalue null)
      (set `PlayerController.bShowMouseCursor` true _returnvalue)
      (bind _returnvalue_2 (`|CreateWidget` "/Game/UI/Network/BP_LobbyWidget.BP_LobbyWidget_C"))
      (`UserWidget.AddToViewport` _returnvalue_2 0))))

(fn `UserConstructionScript`)