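; BP_SubwayCab is a subway cab display actor with configurable numbers, front light beams and doors.
; The construction script applies train and cab numbers to text components and sets visibility and intensity on two spot lights.
; OpenCloseDoors toggles left, right or both sides by DoorsToOpen, snapping front and back doors apart by DoorWidth or back to origin without animation, tracking each side's open state.
; The event graph holds no active logic.
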(fn `Open Close Doors`
  (bind _doorwidth (`self.DoorWidth`))
  (bind _doorwidth_2 (`self.DoorWidth`))
  (bind _doorslf (`self.DoorsLF`))
  (bind _doorslb (`self.DoorsLB`))
  (bind _doorsrf (`self.DoorsRF`))
  (bind _doorsrb (`self.DoorsRB`))
  (switch `/Game/Asset/Map/ModSubwayStation/Blueprints/E_TrainDoorSide` (`self.DoorsToOpen`)
    (:`NewEnumerator0`
      (if (`self.DoorsOpenL`) :!label _label
        (`SceneComponent.K2_SetRelativeLocation` _doorslf (0.0 0.0 0.0) false false)
        (`SceneComponent.K2_SetRelativeLocation` _doorslb (0.0 0.0 0.0) false false)
        (set `self.DoorsOpenL` false)
        (else
          (`SceneComponent.K2_SetRelativeLocation` _doorslf (`KismetMathLibrary.MakeVector` 0.0 _doorwidth) false false)
          (`SceneComponent.K2_SetRelativeLocation` _doorslb (`KismetMathLibrary.MakeVector` 0.0 (* -1 _doorwidth)) false false)
          (set `self.DoorsOpenL` true))))
    (:`NewEnumerator1`
      (if (`self.DoorsOpenR`) :!label _label_2
        (`SceneComponent.K2_SetRelativeLocation` _doorsrf (0.0 0.0 0.0) false false)
        (`SceneComponent.K2_SetRelativeLocation` _doorsrb (0.0 0.0 0.0) false false)
        (set `self.DoorsOpenR` false)
        (else
          (`SceneComponent.K2_SetRelativeLocation` _doorsrf (`KismetMathLibrary.MakeVector` 0.0 _doorwidth_2) false false)
          (`SceneComponent.K2_SetRelativeLocation` _doorsrb (`KismetMathLibrary.MakeVector` 0.0 (* -1 _doorwidth_2)) false false)
          (set `self.DoorsOpenR` true))))
    (:`NewEnumerator2`
      (`|ExecutionSequence`
        (:`then_0`
          (goto _label))
        (:`then_1`
          (goto _label_2))))))

(fn `UserConstructionScript`
  (bind _spotlight1 (`self.SpotLight1`))
  (`TextRenderComponent.K2_SetText` (`self.TextTrainNumber`) (`self.Train Number`))
  (`TextRenderComponent.K2_SetText` (`self.TextCarNumber01`) (`self.Cab Number`))
  (`TextRenderComponent.K2_SetText` (`self.TextCarNumber03`) (`self.Cab Number`))
  (`SceneComponent.SetVisibility` _spotlight1 (`self.Front Light Beams`) false)
  (`SceneComponent.SetVisibility` (`self.SpotLight`) (`self.Front Light Beams`) false)
  (`LightComponent.SetIntensity` _spotlight1 (`self.Front Light Beam Intensity`))
  (`LightComponent.SetIntensity` (`self.SpotLight`) (`self.Front Light Beam Intensity`)))